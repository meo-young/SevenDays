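; BP_3DWidget is a demo Blueprint that shows the VHS camera widget through its Widget component.
; On BeginPlay it casts and caches the Widget_VHS instance, then turns on all of its visibility elements.
; A looping pair of delays toggles the widget's flashlight state every two seconds.
; A timeline meant to drive the battery readout is present but never runs.
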(event EventBeginPlay
  (bind _aswidget_vhs (Utilities|Casting|CastToWidget_VHS (UserInterface|GetWidget (Variables|Default|GetWidget))))
  (bind _output_get (Variables|Default|SetAs%20Widget%20VHS _aswidget_vhs))
  (Default|UpdateVisibility _output_get false true true true true true true)
  (Default|UpdateFlashlight _output_get false :!label _label)
  (Utilities|FlowControl|Delay 2.0)
  (Default|UpdateFlashlight _output_get true)
  (Utilities|FlowControl|Delay 2.0)
  (goto _label))

(fn ConstructionScript)