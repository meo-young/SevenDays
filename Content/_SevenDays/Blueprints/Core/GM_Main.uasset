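; GM_Main, apparently the main game mode, controls Imperfecter screen effects and plays a jump scare.
; GetImperfecter caches effect references from a single Imperfecter instance, looked up by ID.
; SetImperfecterEffect toggles soften, sharpen, compression artifacts and lens distortion together.
; ShowJumpScare briefly enables noise grain and halation with a horror camera shake and a sound at the player pawn, then switches them off after a delay.
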(event Custom|Get%20Imperfecter
  (Variables|Default|SetImperfecterInstance (Class|ImperfecterSubsystem|GetImperfecterInstancebyID (Subsystems|GetImperfecterSubsystem) "IIA_0"))
  (Variables|Default|SetLens%20Distortion (Class|ImperfecterInstanceActor|GetImperfecterEffectbyID (Variables|Default|GetImperfecterInstance) "LensDistortion"))
  (Variables|Default|SetSoften (Class|ImperfecterInstanceActor|GetImperfecterEffectbyID (Variables|Default|GetImperfecterInstance) "Soften"))
  (Variables|Default|SetSharpen (Class|ImperfecterInstanceActor|GetImperfecterEffectbyID (Variables|Default|GetImperfecterInstance) "Sharpen"))
  (Variables|Default|SetCompressionArtifacts (Class|ImperfecterInstanceActor|GetImperfecterEffectbyID (Variables|Default|GetImperfecterInstance) "CompressionArtifacts"))
  (Variables|Default|SetHalation (Class|ImperfecterInstanceActor|GetImperfecterEffectbyID (Variables|Default|GetImperfecterInstance) "Halation"))
  (Variables|Default|SetNoiseGrain (Class|ImperfecterInstanceActor|GetImperfecterEffectbyID (Variables|Default|GetImperfecterInstance) "NoiseGrain")))

(event Custom|SetImperfecterEffect
  (params (bEnable :type Boolean))
  (bind _output_get (Variables|/Script/Imperfecter.ImperfecterEffect|SetbEnabled (Variables|Default|GetSoften) bEnable))
  (bind _output_get_2 (Variables|/Script/Imperfecter.ImperfecterEffect|SetbEnabled (Variables|Default|GetSharpen) _output_get))
  (bind _output_get_3 (Variables|/Script/Imperfecter.ImperfecterEffect|SetbEnabled (Variables|Default|GetCompressionArtifacts) _output_get_2))
  (Variables|/Script/Imperfecter.ImperfecterEffect|SetbEnabled (Variables|Default|GetLens%20Distortion) _output_get_3))

(event EventBeginPlay)

(event EventShowJumpScare
  (Variables|/Script/Imperfecter.ImperfecterEffect|SetbEnabled (Variables|Default|GetNoiseGrain) true)
  (Variables|/Script/Imperfecter.ImperfecterEffect|SetbEnabled (Variables|Default|GetHalation) true)
  (CameraShakes|StartCameraShake (Game|GetPlayerCameraManager 0) "/Game/_SevenDays/Blueprints/CameraShake/CSB_HorrorEffect.CSB_HorrorEffect_C" 1.0 "CameraLocal" "0, 0, 0")
  (Audio|PlaySoundatLocation "/Game/All_In_One_HorrorGame_v1/Mono/Jumpscare/Cue/Jumpscare_Behind_You_Mono_Cue.Jumpscare_Behind_You_Mono_Cue" (Transformation|GetActorLocation (Game|Player|GetPlayerPawn 0)) "0, 0, 0" 1.0 1.0 0.0 0 0 0 0)
  (Utilities|FlowControl|Delay 0.8)
  (Variables|/Script/Imperfecter.ImperfecterEffect|SetbEnabled (Variables|Default|GetNoiseGrain) false)
  (Variables|/Script/Imperfecter.ImperfecterEffect|SetbEnabled (Variables|Default|GetHalation) false)
  (CameraShakes|StopCameraShake (Game|GetPlayerCameraManager 0) 0 true))

(fn ConstructionScript)